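; Base weapon pickup actor that simulates physics in the world and fills its magazine and extra ammo from weapon info by name through a server init event.
; On player overlap, the authority polls until interaction is allowed, then picks a player whose dropped weapon is not this one.
; It offers itself to that player only if their inventory holds no weapon of the same type.
; When a player leaves the sphere, the authority calls SetDropedWeapon on them.
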(event OnComponentBeginOverlap(CollisionSphere)
  (params (OverlappedComponent :type Primitive%20Component%20Object%20Reference) (OtherActor :type Actor%20Object%20Reference) (OtherComp :type Primitive%20Component%20Object%20Reference) (OtherBodyIndex :type Integer) (bFromSweep :type Boolean) (SweepResult :type Hit%20Result%20Structure%20%28by%20ref%29))
  (bind _overlappingactors (Collision|GetOverlappingActors "/Game/Blueprints/Player/BP_PlayerBase.BP_PlayerBase_C" :!class /Script/Engine.Actor))
  ;[0.15 0.15 0.15 0.5] player into collision
  (if (Actor|ActorHasTag OtherActor "Player")
    (Networking|SwitchHasAuthority
      (:Authority
        (if (Variables|Default|GetbCanBeInteractionWith) :!label _label
          (if (> (Utilities|Array|Length _overlappingactors) 1)
            (bind _array_element (Utilities|Array|ForEachLoopwithBreak _overlappingactors :!label _label_2)
              (:LoopBody
                (if (!= (Variables|/Game/Blueprints/Player/BP_PlayerBase.BP_PlayerBase_C|GetDropWeapon _array_element) self)
                  (Variables|Default|SetInteractingPlayer _array_element)
                  (goto _label_2 Break)))
              (:Completed
                (bind _array_element_2 (Utilities|Array|ForEachLoopwithBreak (Variables|/Game/Blueprints/Player/BP_PlayerBase.BP_PlayerBase_C|GetWeaponInventory (Variables|Default|GetInteractingPlayer)) :!label _label_3)
                  (:LoopBody
                    (if (Utilities|Enum|Equal(Enum) (.type (CallFunction|FGetWeaponInfo (Variables|BP_WeaponBase_C|GetWeaponName _array_element_2))) (.type (CallFunction|FGetWeaponInfo (Variables|Default|GetWeaponName))))
                      (Variables|/Game/Blueprints/Player/BP_PlayerBase.BP_PlayerBase_C|SetbCanLootWeapon (Variables|Default|GetInteractingPlayer) false)
                      (goto _label_3 Break)))
                  (:Completed
                    (if (Variables|/Game/Blueprints/Player/BP_PlayerBase.BP_PlayerBase_C|GetbCanLootWeapon (Variables|Default|GetInteractingPlayer))
                      (Default|AddOverlappedWeapons (Variables|Default|GetInteractingPlayer) self)
                      (else
                        (Variables|/Game/Blueprints/Player/BP_PlayerBase.BP_PlayerBase_C|SetbCanLootWeapon (Variables|Default|GetInteractingPlayer) true)))))))
            (else
              (bind _player (Class|INTPlayerBase|GetPlayerRef(Message) (Utilities|Array|Get(acopy) _overlappingactors)))
              (bind _output_get (Variables|Default|SetInteractingPlayer _player))
              (if (!= (Variables|/Game/Blueprints/Player/BP_PlayerBase.BP_PlayerBase_C|GetDropWeapon _output_get) self)
                (goto _label_3))))
          (else
            (Utilities|FlowControl|Delay 0.2)
            (goto _label)))))))

(event OnComponentEndOverlap(CollisionSphere)
  (params (OverlappedComponent :type Primitive%20Component%20Object%20Reference) (OtherActor :type Actor%20Object%20Reference) (OtherComp :type Primitive%20Component%20Object%20Reference) (OtherBodyIndex :type Integer))
  ;[0.15 0.15 0.15 0.5] Player leave collision
  (if (Actor|ActorHasTag OtherActor "Player")
    (Networking|SwitchHasAuthority
      (:Authority
        (bind _player (Class|INTPlayerBase|GetPlayerRef(Message) OtherActor))
        (Default|SetDropedWeapon _player)))))

(event Custom|SRV_Init%20Weapon
  (bind _weaponname (Variables|Default|GetWeaponName))
  (bind _weaponinfo (CallFunction|FGetWeaponInfo _weaponname))
  (bind (_bullethiteffect _bullethitplayereffect _outofammosfx _bulledthitsfx _bullethitplayersfx _maxammoinmag _maxextraammo) (Utilities|Struct|BreakST_WeaponInfo _weaponinfo))
  (Variables|Default|SetCurrentAmmoMag _maxammoinmag)
  (Variables|Default|SetCurrentExtraAmmo _maxextraammo))

(event EventBeginPlay
  ;[0.15 0.15 0.15 0.5] begin
  (Physics|SetSimulatePhysics (Variables|Default|GetWeapon) true)
  (CallFunction|SRVInitWeapon))

(fn ConstructionScript)

(fn GetWeaponRef
  (return self))