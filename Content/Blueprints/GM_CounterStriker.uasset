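; GM_CounterStriker is the game mode for a Counter-Strike-style team game that handles player spawning.
; On PostLogin it records each joining controller in ConnectedPlayers and caches all terrorist and counter-terrorist spawn point actors.
; RequestPlayerSpwan picks a random spawn point transform for the requested team and tells that player controller to spawn with it.
; GetGameModeRef returns the game mode itself.
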(event Custom|RequestPlayerSpwan
  (params (PlayerController :type PC%20Counter%20Strike%20Object%20Reference) (Team :type Actor%20Class%20Reference))
  (Default|SpawnPlayer PlayerController Team (Math|Transform|SelectTransform (Transformation|GetActorTransform (.OutItem (Utilities|Array|Random (Variables|Default|GetTerroristSpawnPoints)))) (Transformation|GetActorTransform (.OutItem (Utilities|Array|Random (Variables|Default|GetCounterTerroristSpawnPoints)))) (== Team "/Game/Blueprints/Player/BP_Terrorists.BP_Terrorists_C"))))

(event EventTick
  (params (DeltaSeconds :type Float%20%28single-precision%29)))

(event EventPostLogin
  (params (NewPlayer :type Player%20Controller%20Object%20Reference))
  (Utilities|Array|AddUnique (Variables|Default|GetConnectedPlayers) NewPlayer)
  (bind _outactors (Actor|GetAllActorsOfClass "/Game/Blueprints/spawnPoints/BP_spawnPointCounterTerrorist.BP_spawnPointCounterTerrorist_C"))
  (Variables|Default|SetCounterTerroristSpawnPoints _outactors)
  (bind _outactors_2 (Actor|GetAllActorsOfClass "/Game/Blueprints/spawnPoints/BP_spawnPointTerrorist.BP_spawnPointTerrorist_C"))
  (Variables|Default|SetTerroristSpawnPoints _outactors_2))

(fn ConstructionScript)

(fn GetGameModeRef
  (return self))