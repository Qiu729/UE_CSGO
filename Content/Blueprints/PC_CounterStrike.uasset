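; Player controller for a Counter-Strike-style game that handles team selection, pawn spawning and the player's HUD.
; BeginPlay shows the team menu over a level camera with UI-only input; the chosen team goes through a server event to the GameMode as a spawn request.
; SpawnPlayer spawns and possesses the team's pawn, then a client event switches to HUD, crosshair and game input.
; Widgets are created on first show and cached.
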(event Custom|ShowHideWidget
  (params (Widget :type E_GameWidgets%20Enum :default "NewEnumerator0") (bShow :type Boolean))
  (CallFunction|CLShowHideWidget Widget bShow))

(event Custom|CL_ShowHideWidget
  (params (Widget :type E_GameWidgets%20Enum :default "NewEnumerator0") (bShow :type Boolean))
  (if bShow
    (CallFunction|FShowWidget Widget true)
    (else
      (CallFunction|FHideWidget Widget false))))

(event Custom|SpawnPlayer
  (params (Team :type Actor%20Class%20Reference) (SpawnTransform :type Transform))
  (bind _returnvalue (Game|SpawnActorfromClass Team SpawnTransform "Undefined" "MultiplyWithRoot" 0 0))
  (bind _output_get (Variables|Default|SetPlayerPawn _returnvalue))
  (bind _player (Class|INTPlayerBase|GetPlayerRef(Message) _output_get))
  (Pawn|Possess _player)
  (CallFunction|CLSpawnPlayer))

(event Custom|SelectTeam
  (params (Team :type Actor%20Class%20Reference))
  (CallFunction|SRVSelectTeam Team))

(event Custom|SRV_SelectTeam
  (params (Team :type Actor%20Class%20Reference))
  (Default|RequestPlayerSpwan (Variables|Default|GetGame%20Mode) self Team))

(event Custom|CL_spawnPlayer
  (CallFunction|ShowHideWidget "NewEnumerator0" false)
  (CallFunction|ShowHideWidget "NewEnumerator1" true)
  (CallFunction|ShowHideWidget "NewEnumerator2" true)
  (Input|SetInputModeGameOnly self false)
  (Variables|Default|SetbShowMouseCursor false))

(event EventBeginPlay
  (CallFunction|ShowHideWidget "NewEnumerator0" true)
  (bind _gamemode (Class|INTGameMode|GetGameModeRef(Message) (Game|GetGameMode)))
  (Variables|Default|SetGame%20Mode _gamemode)
  (bind _returnvalue (Actor|GetActorOfClass "/Script/Engine.CameraActor"))
  (Game|Player|SetViewTargetwithBlend _returnvalue 0.0 "VTBlend_Linear" 0.0 false)
  (Input|SetInputModeUIOnly self 0 "DoNotLock" false)
  (Variables|Default|SetbShowMouseCursor true))

(fn ConstructionScript)

(fn FShowWidget
  (params (Widget :type E_GameWidgets%20Enum :default "NewEnumerator0") (bShow :type Boolean))
  (switch Utilities|FlowControl|Switch|SwitchonE_GameWidgets Widget
    (:NewEnumerator0
      (Variables|Default|GetWB_TeamSelection
        (:then
          _)
        (:else
          (bind _returnvalue (UserInterface|CreateWidget "/Game/UI/WB_TeamSelection.WB_TeamSelection_C"))
          (bind _output_get (Variables|Default|SetWB_TeamSelection _returnvalue))))
      (UserInterface|Viewport|AddtoViewport _output_get 0))
    (:NewEnumerator1
      (Variables|Default|GetWB_Main
        (:then
          _)
        (:else
          (bind _returnvalue_2 (UserInterface|CreateWidget "/Game/UI/WB_Main.WB_Main_C"))
          (bind _output_get_2 (Variables|Default|SetWB_Main _returnvalue_2))))
      (UserInterface|Viewport|AddtoViewport _output_get_2 0))
    (:NewEnumerator2
      (Variables|Default|GetWB_CrossHair
        (:then
          _)
        (:else
          (bind _returnvalue_3 (UserInterface|CreateWidget "/Game/UI/WB_CrossHair.WB_CrossHair_C"))
          (bind _output_get_3 (Variables|Default|SetWB_CrossHair _returnvalue_3))))
      (UserInterface|Viewport|AddtoViewport _output_get_3 0))))

(fn FHideWidget
  (params (Widget :type E_GameWidgets%20Enum :default "NewEnumerator0") (bShow :type Boolean))
  (switch Utilities|FlowControl|Switch|SwitchonE_GameWidgets Widget
    (:NewEnumerator0
      (bind _wb_teamselection (Variables|Default|GetWB_TeamSelection)
        (:then
          (Widget|RemovefromParent _wb_teamselection))
        (:else)))
    (:NewEnumerator1
      (bind _wb_main (Variables|Default|GetWB_Main)
        (:then
          (Widget|RemovefromParent _wb_main))
        (:else)))
    (:NewEnumerator2
      (bind _wb_crosshair (Variables|Default|GetWB_CrossHair)
        (:then
          (Widget|RemovefromParent _wb_crosshair))
        (:else)))))

(fn GetGameModeRef
  (return 0))

(fn GetPlayerControllerRef
  (return self))